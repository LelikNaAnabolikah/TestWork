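; BP_GameController switches the UI between a start window and a main view, and records tile selections.
; After a short delay, Init shows WBP_StartWindow, whose ShowMenu event swaps it for WBP_MainView, both in UI-only input mode.
; SaveTile and RemoveTile update the SelectedTile map, then close the main view and recreate the start window.
; RemoveTile writes a "-1" sentinel for the key instead of deleting the entry.
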(event `self.ReceiveInit`
  (`KismetSystemLibrary.Delay` 0.2)
  (`self.ShowStartWindow`))

(event `ShowStartWindow`
  (bind _returnvalue (`GameplayStatics.GetPlayerController` 0))
  (bind _returnvalue_2 (`|CreateWidget` "/Game/Widgets/WBP_StartWindow.WBP_StartWindow_C"))
  (bind _output_get (set `self.startWindow` _returnvalue_2))
  (add `/Game/Widgets/WBP_StartWindow.ShowMenu` _output_get (delegate `ShowMenu_Event_0`))
  (`UserWidget.AddToViewport` _output_get 0)
  (`WidgetBlueprintLibrary.SetInputMode_UIOnlyEx` _returnvalue _output_get "LockAlways")
  (set `PlayerController.bShowMouseCursor` false _returnvalue))

(event `ShowMenu_Event_0`
  (`Widget.RemoveFromParent` (`self.startWindow`))
  (bind _returnvalue (`|CreateWidget` "/Game/Widgets/WBP_MainView.WBP_MainView_C"))
  (bind _output_get (set `self.ref` _returnvalue))
  (`UserWidget.AddToViewport` _output_get 0)
  (`WidgetBlueprintLibrary.SetInputMode_UIOnlyEx` (`GameplayStatics.GetPlayerController` 0) _output_get "LockAlways"))

(fn `RemoveTile`
  (params (Key :type "Integer (by ref)"))
  (`BlueprintMapLibrary.Map_Add` (`self.SelectedTile`) Key "-1")
  (`Widget.RemoveFromParent` (`self.ref`))
  (`self.ShowStartWindow`))

(fn `SaveTile`
  (params (Key :type "Integer (by ref)") (Value :type "Name (by ref)"))
  (`BlueprintMapLibrary.Map_Add` (`self.SelectedTile`) Key Value)
  (`Widget.RemoveFromParent` (`self.ref`))
  (`self.ShowStartWindow`))